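; BP_EasyPortal is a placeable portal actor that wraps the BPCompEasyPortal component and links it to an OutPortal.
; The construction script initializes the component with the render plane mesh, an out-direction debug arrow, and activation and teleport triggers, then sets its OutPortal.
; GetEasyPortalComponent re-applies OutPortal before returning the component.
; The event graph holds only disabled placeholder events, so the actor itself adds no runtime event logic.
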(event EventBeginPlay)

(event Collision|EventActorBeginOverlap
  (params (OtherActor :type Actor%20Object%20Reference)))

(event EventTick
  (params (DeltaSeconds :type Float%20%28single-precision%29)))

(fn ConstructionScript
  (Default|Init (Variables|Default|GetBPComp_EasyPortal) (Variables|Default|GetRenderPlaneMesh) (Variables|Default|GetPortalOutDirectionDebugArrow) (Variables|Default|GetActivationTrigger) (Variables|Default|GetTeleportTrigger))
  (Variables|/EasyPortals/Core/BPComp_EasyPortal.BPComp_EasyPortal_C|SetOutPortal (Variables|Default|GetBPComp_EasyPortal) (Variables|Default|GetOutPortal)))

(fn GetEasyPortalComponent
  (bind _bpcomp_easyportal (Variables|Default|GetBPComp_EasyPortal))
  (Variables|/EasyPortals/Core/BPComp_EasyPortal.BPComp_EasyPortal_C|SetOutPortal _bpcomp_easyportal (Variables|Default|GetOutPortal))
  (return _bpcomp_easyportal))